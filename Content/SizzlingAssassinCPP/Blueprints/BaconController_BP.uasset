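; BaconController_BP is a controller Blueprint that handles pausing and mouse cursor visibility.
; On BeginPlay it shows the cursor if the current level is MainMenuMap.
; The P key drives a FlipFlop that toggles game pause, adding PauseMenuWidget_BP with the cursor shown when paused.
; On unpause it hides the cursor and removes the pause widget, found through a widget class search.
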(event EventBeginPlay
  (bind _returnvalue (Game|GetCurrentLevelName true))
  (if (Utilities|Enum|Equal(Enum) "MainMenuMap" _returnvalue)
    (Variables|Default|SetbShowMouseCursor true)))

(event EventTick
  (params (DeltaSeconds :type Float%20%28single-precision%29)))

(event Input|KeyboardEvents|P
  (params (Key :type Key%20Structure))
  (:Pressed
    (bind _isa (Utilities|FlowControl|FlipFlop)
      (:A
        _)
      (:B
        _))
    (Game|SetGamePaused _isa)
    (if (Game|IsGamePaused)
      (bind _returnvalue (UserInterface|CreateWidget "/Game/SizzlingAssassinCPP/Blueprints/PauseMenuWidget_BP.PauseMenuWidget_BP_C"))
      (UserInterface|Viewport|AddtoViewport _returnvalue 0)
      (Variables|Default|SetbShowMouseCursor true)
      (else
        (Variables|Default|SetbShowMouseCursor false)
        (bind _foundwidgets (Widget|GetAllWidgetsOfClass "/Game/SizzlingAssassinCPP/Blueprints/PauseMenuWidget_BP.PauseMenuWidget_BP_C" true))
        (Widget|RemovefromParent _foundwidgets)))))

(fn ConstructionScript)